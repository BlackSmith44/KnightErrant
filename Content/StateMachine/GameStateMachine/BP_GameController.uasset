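; BP_GameController drives the game's state machine, holding the current state actor and the main view widget.
; On BeginPlay it runs a setup chain that creates and stores WBP_MainView for the first player, then spawns BP_MenuState as the initial state.
; ChangeState destroys the previous state actor, if valid, and stores the new one.
; An unreachable SetGameController call remains as leftover logic.
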(event `self.ReceiveBeginPlay`
  (bind _returnvalue (`|CreateWidget` "/Game/Widgets/Views/WBP_MainView.WBP_MainView_C" (`GameplayStatics.GetPlayerController` 0)))
  (set `self.MainView` _returnvalue)
  (bind _returnvalue_2 (`|SpawnActorFromClass` "/Game/StateMachine/GameStateMachine/BP_MenuState.BP_MenuState_C" (`KismetMathLibrary.Conv_VectorToTransform` (`KismetMathLibrary.Vector_Zero`)) "AlwaysSpawn" "MultiplyWithRoot" null null))
  (`self.Change State` _returnvalue_2))

(fn `Change State`
  (params (newState :type "/Game/StateMachine/GameStateMachine/BP_BaseState Object Reference"))
  (bind _currentstate (`self.currentState`))
  (if (`KismetSystemLibrary.IsValid` _currentstate)
    (`self.K2_DestroyActor` _currentstate))
  (set `self.currentState` newState))

(fn `UserConstructionScript`)