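; BP_PauseState is the game state machine's pause state, an actor that runs the pause menu.
; On BeginPlay it shows the GameController's PauseView, enables input and binds the view's dispatchers to switch to BP_GameState or BP_StartState.
; When destroyed, it hides the view and disables input.
; The C key only prints a debug string, and an unconnected WIP chain would add the IMC_Pause Enhanced Input mapping context.
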(event `self.ReceiveBeginPlay`
  (bind _pauseview (`/Game/StateMachine/GameStateMachine/BP_GameController.PauseView` (`self.GameController`)))
  (`parent.ReceiveBeginPlay`)
  (`KismetSystemLibrary.PrintString` "MenuState says Hello")
  (`/Game/Widgets/Views/WBP_PauseView.ShowView` _pauseview)
  (add `/Game/Widgets/Views/WBP_PauseView.DispatcherChangeToGameState` _pauseview (delegate `StartGame`))
  (add `/Game/Widgets/Views/WBP_PauseView.DispatcherChangeToStartState` _pauseview (delegate `BackToStart`))
  (`self.EnableInput` (`/Game/StateMachine/GameStateMachine/BP_GameController.PlayerControl` (`self.GameController`))))

(event `StartGame`
  (`self.ChangeThisState` "/Game/StateMachine/GameStateMachine/BP_GameState.BP_GameState_C"))

(event `BackToStart`
  (`self.ChangeThisState` "/Game/StateMachine/GameStateMachine/BP_StartState.BP_StartState_C"))

(event `self.ReceiveDestroyed`
  (`/Game/Widgets/Views/WBP_PauseView.Hide View` (`/Game/StateMachine/GameStateMachine/BP_GameController.PauseView` (`self.GameController`)))
  (`self.DisableInput` (`/Game/StateMachine/GameStateMachine/BP_GameController.PlayerControl` (`self.GameController`))))

(event `Key|C` :paused true
  (params (Key :type "Key Structure"))
  (:`Pressed`
    (`KismetSystemLibrary.PrintString` "YYYYYYYYYYYYYYYYYYYYYYYYYYYYYYY")))

(fn `UserConstructionScript`
  (`parent.UserConstructionScript`))