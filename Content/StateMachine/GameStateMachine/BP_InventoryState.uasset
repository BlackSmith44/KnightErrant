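; BP_InventoryState is the game state machine state that is active while the inventory is open.
; On BeginPlay it shows the GameController's InventoryView and binds the view's ChangeToGameState dispatcher to resume play.
; Resuming spawns a BP_GameState actor and passes it to GameController.ChangeState, so each state is its own actor.
; When this state is destroyed, it hides the inventory view.
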(event `self.ReceiveBeginPlay`
  (bind _inventoryview (`/Game/StateMachine/GameStateMachine/BP_GameController.InventoryView` (`self.GameController`)))
  (`parent.ReceiveBeginPlay`)
  (`KismetSystemLibrary.PrintString` "INVENTORY")
  (`/Game/Widgets/Views/WBP_InventoryView.ShowView` _inventoryview)
  (add `/Game/Widgets/Views/WBP_InventoryView.DispatcherChangeToGameState` _inventoryview (delegate `ResumeGame`)))

(event `ResumeGame`
  (bind _returnvalue (`|SpawnActorFromClass` "/Game/StateMachine/GameStateMachine/BP_GameState.BP_GameState_C" (`KismetMathLibrary.Conv_VectorToTransform` (`KismetMathLibrary.Vector_Zero`)) "AlwaysSpawn" "MultiplyWithRoot" null null))
  (`/Game/StateMachine/GameStateMachine/BP_GameController.Change State` (`self.GameController`) _returnvalue))

(event `self.ReceiveDestroyed`
  (`/Game/Widgets/Views/WBP_InventoryView.HideView` (`/Game/StateMachine/GameStateMachine/BP_GameController.InventoryView` (`self.GameController`))))

(fn `UserConstructionScript`
  (`parent.UserConstructionScript`))