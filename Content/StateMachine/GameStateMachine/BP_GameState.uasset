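; Gameplay state in a custom game state machine, active while the HUD is on screen.
; On BeginPlay it shows the GameController's HUD view through a macro and binds its dispatchers to switch to the inventory, pause or lose state via ChangeThisState.
; Destroying the state hides the HUD view.
; Unconnected WIP nodes sketch adding and removing the default Enhanced Input mapping context.
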(event `self.ReceiveBeginPlay`
  (bind _hudview (`/Game/StateMachine/GameStateMachine/BP_GameController.HUDView` (`self.GameController`)))
  (`parent.ReceiveBeginPlay`)
  (`KismetSystemLibrary.PrintString` "GameState says hello")
  (`/Game/Widgets/Views/WBP_HUDView.ShowView` _hudview)
  (add `/Game/Widgets/Views/WBP_HUDView.DispatcherChangeToInventoryState` _hudview (delegate `OpenInventory`))
  (add `/Game/Widgets/Views/WBP_HUDView.DispatcherChangeToPauseState` _hudview (delegate `OpenPauseMenu`))
  (add `/Game/Widgets/Views/WBP_HUDView.DispatcherChangeToLoseState` _hudview (delegate `OpenLoseState`)))

(event `OpenInventory`
  (`self.ChangeThisState` "/Game/StateMachine/GameStateMachine/BP_InventoryState.BP_InventoryState_C"))

(event `OpenPauseMenu`
  (`self.ChangeThisState` "/Game/StateMachine/GameStateMachine/BP_PauseState.BP_PauseState_C"))

(event `OpenLoseState`
  (`self.ChangeThisState` "/Game/StateMachine/GameStateMachine/BP_LoseState.BP_LoseState_C"))

(event `self.ReceiveDestroyed`
  (`/Game/Widgets/Views/WBP_HUDView.Hide View` (`/Game/StateMachine/GameStateMachine/BP_GameController.HUDView` (`self.GameController`))))

(fn `UserConstructionScript`
  (`parent.UserConstructionScript`))