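; BP_StartState is the start-menu state in the game's state machine, shown before a new game begins.
; On BeginPlay it shows the GameController's StartView and binds StartGame to that view's new-game dispatcher.
; StartGame spawns a BP_GameState actor and hands it to GameController.ChangeState.
; States are spawned actors, so this one hides the StartView when it is destroyed.
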(event `self.ReceiveBeginPlay`
  (bind _startview (`/Game/StateMachine/GameStateMachine/BP_GameController.StartView` (`self.GameController`)))
  (`parent.ReceiveBeginPlay`)
  (`KismetSystemLibrary.PrintString` "START THE GAME")
  (`/Game/Widgets/Views/WBP_StartView.ShowView` _startview)
  (add `/Game/Widgets/Views/WBP_StartView.DispatcherStartNewGame` _startview (delegate `StartGame`)))

(event `StartGame`
  (bind _returnvalue (`|SpawnActorFromClass` "/Game/StateMachine/GameStateMachine/BP_GameState.BP_GameState_C" (`KismetMathLibrary.Conv_VectorToTransform` (`KismetMathLibrary.Vector_Zero`)) "AlwaysSpawn" "MultiplyWithRoot" null null))
  (`/Game/StateMachine/GameStateMachine/BP_GameController.Change State` (`self.GameController`) _returnvalue))

(event `self.ReceiveDestroyed`
  (`/Game/Widgets/Views/WBP_StartView.HideView` (`/Game/StateMachine/GameStateMachine/BP_GameController.StartView` (`self.GameController`))))

(fn `UserConstructionScript`
  (`parent.UserConstructionScript`))