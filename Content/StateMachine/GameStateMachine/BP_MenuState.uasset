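; BP_MenuState is the game state machine's menu state, an actor that displays the pause menu while active.
; On BeginPlay it shows the GameController's PauseMenuView and binds that view's change-to-game-state dispatcher to StartGame.
; StartGame spawns a BP_GameState actor and passes it to GameController.ChangeState.
; When the menu state is destroyed, it hides the pause menu view.
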(event `self.ReceiveBeginPlay`
  (bind _pausemenuview (`/Game/StateMachine/GameStateMachine/BP_GameController.PauseMenuView` (`self.GameController`)))
  (`parent.ReceiveBeginPlay`)
  (`KismetSystemLibrary.PrintString` "MenuState says Hello")
  (`/Game/Widgets/Views/WBP_PauseMenuView.ShowView` _pausemenuview)
  (add `/Game/Widgets/Views/WBP_PauseMenuView.EventD ChangeToGameState` _pausemenuview (delegate `StartGame`)))

(event `StartGame`
  (bind _returnvalue (`|SpawnActorFromClass` "/Game/StateMachine/GameStateMachine/BP_GameState.BP_GameState_C" (`KismetMathLibrary.Conv_VectorToTransform` (`KismetMathLibrary.Vector_Zero`)) "AlwaysSpawn" "MultiplyWithRoot" null null))
  (`/Game/StateMachine/GameStateMachine/BP_GameController.Change State` (`self.GameController`) _returnvalue))

(event `self.ReceiveDestroyed`
  (`/Game/Widgets/Views/WBP_PauseMenuView.Hide View` (`/Game/StateMachine/GameStateMachine/BP_GameController.PauseMenuView` (`self.GameController`))))

(fn `UserConstructionScript`
  (`parent.UserConstructionScript`))