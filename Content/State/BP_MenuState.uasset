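; BP_MenuState is a state Blueprint, named for the menu, that currently holds only a debug readout.
; On BeginPlay it calls its parent, finds the BP_GameController actor in the level and prints that actor's Test value as text.
; Its Init override and construction script only forward to the parent, and the overlap and Tick events are disabled placeholders.
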(event `self.ReceiveBeginPlay`
  (`parent.ReceiveBeginPlay`)
  (bind _returnvalue (`GameplayStatics.GetActorOfClass` "/Game/State/BP_GameController.BP_GameController_C"))
  (`KismetSystemLibrary.PrintText` (`KismetTextLibrary.Conv_IntToText` (`/Game/State/BP_GameController.test` _returnvalue))))

(fn `Init`
  (`parent.Init`))

(fn `UserConstructionScript`
  (`parent.UserConstructionScript`))