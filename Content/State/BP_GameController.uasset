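; BP_GameController is an Actor Blueprint that runs a simple state machine for the game, starting in the menu state.
; On BeginPlay it constructs a BP_MenuState object and passes it to ChangeState.
; ChangeState calls DestroyState on any valid current state, stores the new one, then calls its Init with the controller as context.
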(event `self.ReceiveBeginPlay`
  (bind _returnvalue (`|GenericCreateObject` "/Game/State/BP_MenuState.BP_MenuState_C"))
  (`self.Change State` _returnvalue))

(fn `Change State`
  (params (newState :type "/Game/State/BP_BaseState Object Reference"))
  (bind _currentstate (`self.currentState`))
  (if (`KismetSystemLibrary.IsValid` _currentstate)
    (`/Game/State/BP_BaseState.DestroyState` _currentstate))
  (bind _output_get (set `self.currentState` newState))
  (if (`KismetSystemLibrary.IsValid` _output_get)
    (`/Game/State/BP_BaseState.Init` _output_get self)))

(fn `UserConstructionScript`)