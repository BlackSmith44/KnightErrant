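; BP_MenuState is the main menu state in an actor-based game state machine driven by a GameController.
; On BeginPlay it creates the WBP_MainMenu widget, shows the mouse cursor and binds the widget's change-to-game-state dispatcher to StartGame.
; StartGame spawns a BP_GameState actor and hands it to the GameController's ChangeState.
; When destroyed, it removes the menu, forces garbage collection and hides the cursor.
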(event `self.ReceiveBeginPlay`
  (bind _returnvalue (`GameplayStatics.GetPlayerController` 0))
  (`parent.ReceiveBeginPlay`)
  (bind _returnvalue_2 (`|CreateWidget` "/Game/Widgets/Views/WBP_MainMenu.WBP_MainMenu_C" _returnvalue))
  (bind _output_get (set `self.MainView` _returnvalue_2))
  (set `PlayerController.bShowMouseCursor` true _returnvalue)
  (`UserWidget.AddToViewport` _returnvalue_2 0)
  (add `/Game/Widgets/Views/WBP_MainMenu.EventD ChangeToGameState` _output_get (delegate `StartGame`)))

(event `StartGame`
  (bind _returnvalue (`|SpawnActorFromClass` "/Game/Blueprints/State/BP_GameState.BP_GameState_C" (`KismetMathLibrary.Conv_VectorToTransform` (`KismetMathLibrary.Vector_Zero`)) "AlwaysSpawn" "MultiplyWithRoot" null null))
  (`/Game/Blueprints/State/BP_GameController.Change State` (`self.GameController`) _returnvalue))

(event `self.ReceiveDestroyed`
  ;[1 1 1] This shouldn't be here either
  (`Widget.RemoveFromParent` (`self.MainView`))
  (`KismetSystemLibrary.CollectGarbage`)
  (set `PlayerController.bShowMouseCursor` false (`GameplayStatics.GetPlayerController` 0)))

(fn `DestroyState`
  (`parent.DestroyState`))

(fn `Init`
  (params (gameController :type "/Game/Blueprints/State/BP_GameController Object Reference"))
  (`parent.Init` gameController)
  (`KismetSystemLibrary.PrintString` "MenuState says Hello"))

(fn `Tick`
  (`parent.Tick`))

(fn `UserConstructionScript`
  (`parent.UserConstructionScript`))